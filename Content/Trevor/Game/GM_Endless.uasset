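; GM_Endless is the game mode for an endless driving game, tracking distance travelled and handling the game-over screen.
; On begin play it fades the camera in, shows the WBP_UI HUD and starts a looping distance timer.
; Each tick adds the BP_PawnCar's SpeedModifier to Distance and updates the HUD.
; Once IsGameOver is set, the next tick pauses the game and shows WBP_PlayAgain with the final distance.
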(event `self.ReceiveBeginPlay`
  (bind _returnvalue (`GameplayStatics.GetPlayerController` 0))
  (`WidgetBlueprintLibrary.SetInputMode_GameOnly` _returnvalue)
  (set `PlayerController.bShowMouseCursor` false _returnvalue)
  (`PlayerCameraManager.StartCameraFade` :`self` (`PlayerController.PlayerCameraManager` _returnvalue) :`FromAlpha` 1.0 :`ToAlpha` 0.0 :`Duration` 5.0 :`bShouldFadeAudio` true)
  (bind _returnvalue_2 (`|CreateWidget` "/Game/Trevor/Game/WBP_UI.WBP_UI_C"))
  (bind _output_get (set `self.ScreenUI` _returnvalue_2))
  (`UserWidget.AddToViewport` _output_get 0)
  (`/Game/Trevor/Game/WBP_UI.UpdateDist` _output_get (`self.Distance`))
  (`KismetSystemLibrary.K2_SetTimerDelegate` (delegate `IncreaseDistance`) (`self.DistanceRoI`) true))

(event `IncreaseDistance`
  (bind _returnvalue (`GameplayStatics.GetPlayerController` 0))
  (bind _distance (`self.Distance`))
  (if (`self.IsGameOver?`)
    (`GameplayStatics.SetGamePaused` true)
    (`WidgetLayoutLibrary.RemoveAllWidgets`)
    (bind _returnvalue_2 (`|CreateWidget` "/Game/Trevor/Game/WBP_PlayAgain.WBP_PlayAgain_C"))
    (bind _output_get (set `self.EndScreen` _returnvalue_2))
    (`/Game/Trevor/Game/WBP_PlayAgain.UpdateEndDistance` _output_get _distance)
    (`UserWidget.AddToViewport` _output_get 0)
    (`WidgetBlueprintLibrary.SetInputMode_UIOnlyEx` _returnvalue null)
    (set `PlayerController.bShowMouseCursor` true _returnvalue)
    (else
      (bind _returnvalue_3 (`GameplayStatics.GetActorOfClass` "/Game/Trevor/Car/BP_PawnCar.BP_PawnCar_C"))
      (bind _output_get_2 (set `self.Distance` (+ (`/Game/Trevor/Car/BP_PawnCar.SpeedModifier` _returnvalue_3) _distance 0.0)))
      (`/Game/Trevor/Game/WBP_UI.UpdateDist` (`self.ScreenUI`) _output_get_2))))

(fn `UserConstructionScript`)