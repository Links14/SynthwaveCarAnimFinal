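; BP_PawnCar is the player car pawn for what appears to be an endless runner, shifting between three lanes with A/D via timelines.
; Looping timers raise SpeedModifier and cycle six toon-shader color pairs, crossfaded on a dynamic post-process material that the construction script adds to the CineCamera.
; DestroySphere overlaps count destroyed roads, though distance-based recoloring is unwired.
; BP_Ballard collisions call SetGamePaused with false.
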(event `CenterToLeft`
  (bind _skm_sportscar (`self.SKM_SportsCar`))
  (bind (_relativelocation_x _relativelocation_y _relativelocation_z) (`KismetMathLibrary.BreakVector` (`SceneComponent.RelativeLocation` _skm_sportscar)))
  ;[1 1 1] Movement
  (bind (_direction _moveleft) (`Timeline|movementLeft` :!label _label)
    (:`Update`
      (`SceneComponent.K2_SetRelativeTransform` _skm_sportscar (`KismetMathLibrary.MakeTransform` (`KismetMathLibrary.MakeVector` _moveleft _relativelocation_y _relativelocation_z) (`SceneComponent.RelativeRotation` _skm_sportscar) (`SceneComponent.RelativeScale3D` _skm_sportscar)) false false))))

(event `Key|A`
  (params (Key :type "Key Structure"))
  ;[1 1 1] Movement
  (:`Pressed`
    (if (`self.IsRight`)
      (set `self.IsRight` false)
      (`self.CenterFromRIght`)
      (elif (not (`self.IsLeft`))
        (set `self.IsLeft` true)
        (`self.CenterToLeft`)))))

(event `CenterFromleft`
  ;[1 1 1] Movement
  (goto _label :!via `Reverse`))

(event `CenterToRight`
  (bind _skm_sportscar (`self.SKM_SportsCar`))
  (bind (_relativelocation_x _relativelocation_y _relativelocation_z) (`KismetMathLibrary.BreakVector` (`SceneComponent.RelativeLocation` _skm_sportscar)))
  ;[1 1 1] Movement
  (bind (_direction _moveright) (`Timeline|movementRight` :!label _label_2)
    (:`Update`
      (`SceneComponent.K2_SetRelativeTransform` _skm_sportscar (`KismetMathLibrary.MakeTransform` (`KismetMathLibrary.MakeVector` _moveright _relativelocation_y _relativelocation_z) (`SceneComponent.RelativeRotation` _skm_sportscar) (`SceneComponent.RelativeScale3D` _skm_sportscar)) false false))))

(event `Key|D`
  (params (Key :type "Key Structure"))
  ;[1 1 1] Movement
  (:`Pressed`
    (if (`self.IsLeft`)
      (set `self.IsLeft` false)
      (`self.CenterFromleft`)
      (elif (not (`self.IsRight`))
        (set `self.IsRight` true)
        (`self.CenterToRight`)))))

(event `CenterFromRIght`
  ;[1 1 1] Movement
  (goto _label_2 :!via `Reverse`))

(event `self.BoxCollision.OnComponentBeginOverlap`
  (params (OverlappedComponent :type "PrimitiveComponent Object Reference") (OtherActor :type "Actor Object Reference") (OtherComp :type "PrimitiveComponent Object Reference") (OtherBodyIndex :type Integer) (bFromSweep :type Boolean) (SweepResult :type "HitResult Structure (by ref)"))
  ;[1 1 1] When collision occurs
  (cast `/Game/Trevor/Road/BP_Ballard` OtherActor)
  (`GameplayStatics.SetGamePaused` false))

(event `self.ReceiveBeginPlay`
  ;[1 1 1] Begin Play Events
  (`self.SetGameSpeedByTime`)
  (`self.SetColorByTime`))

(event `self.DestroySphere.OnComponentBeginOverlap`
  (params (OverlappedComponent :type "PrimitiveComponent Object Reference") (OtherActor :type "Actor Object Reference") (OtherComp :type "PrimitiveComponent Object Reference") (OtherBodyIndex :type Integer) (bFromSweep :type Boolean) (SweepResult :type "HitResult Structure (by ref)"))
  ;[1 1 1] Calculate number of roads destroyed, as well as (depreciated) change color by distance
  (set `self.RoadsDestroyed` (+ 1 (`self.RoadsDestroyed`))))

(event `SetColorByTime`
  ;[1 1 1] Set
  (`KismetSystemLibrary.K2_SetTimerDelegate` (delegate `SetIndexes`) 10.0 true))

(event `SetIndexes`
  (bind _toonshader (`self.ToonShader`))
  (bind _pplist (`self.PPlist`))
  (bind _ppindex (`self.PPindex`))
  (bind _ppindex_2 (`self.PPindex`))
  (bind (_output_light _output_shadow) (break `/Game/Trevor/Stuct_Color` (`|GetArrayItem` _pplist _ppindex_2)))
  (bind (_output_light_2 _output_shadow_2) (break `/Game/Trevor/Stuct_Color` (`|GetArrayItem` _pplist (mod (+ _ppindex_2 1) 6))))
  ;[1 1 1] Set
  (if (>= _ppindex 5)
    (set `self.PPindex` 0)
    ;[1 1 1] Sets the new colors and plays the animations when it does so
    (bind (_direction _fade) (`Timeline|Timeline` :!via `PlayFromStart` :!label _label_3)
      (:`Update`
        (`MaterialInstanceDynamic.SetVectorParameterValue` _toonshader "ShadowTint" (`KismetMathLibrary.LinearColorLerp` _output_shadow _output_shadow_2 _fade))
        (`MaterialInstanceDynamic.SetVectorParameterValue` _toonshader "WhiteTint" (`KismetMathLibrary.LinearColorLerp` _output_light _output_light_2 _fade))))
    (else
      (set `self.PPindex` (+ _ppindex 1))
      (goto _label_3 :!via `PlayFromStart`))))

(event `SetGameSpeedByTime`
  ;[1 1 1] Set speed by time
  (`KismetSystemLibrary.K2_SetTimerDelegate` (delegate `GameSpeed`) (`self.Speed+bySeconds`) true))

(event `GameSpeed`
  ;[1 1 1] Set speed by time
  (set `self.SpeedModifier` (+ (`self.SpeedModifier`) 0.1)))

(fn `UserConstructionScript`
  (bind (_output_light _output_shadow) (break `/Game/Trevor/Stuct_Color` (`|GetArrayItem` (`self.PPlist`))))
  (bind _weightedblendables_array (break `WeightedBlendables` (break `PostProcessSettings` (`CameraComponent.PostProcessSettings` (`self.CineCamera`)))))
  (bind _returnvalue (`KismetMaterialLibrary.CreateDynamicMaterialInstance` "/Game/Trevor/MasterMaterials/PP_ToonShader.PP_ToonShader"))
  (bind _output_get (set `self.ToonShader` _returnvalue))
  (`KismetArrayLibrary.Array_Add` _weightedblendables_array (make `WeightedBlendable` 1.0 _output_get))
  (`MaterialInstanceDynamic.SetVectorParameterValue` _output_get "ShadowTint" _output_shadow)
  (`MaterialInstanceDynamic.SetVectorParameterValue` _output_get "WhiteTint" _output_light))