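; BP_Ballard is a road obstacle actor that scrolls with the road and removes itself once it is far out of range.
; Each Tick it looks up the BP_Road actor, reads its Speed and moves along local Y by that amount per frame, without delta-time scaling.
; It destroys itself when the world X of its Ballards component drops below a negative cutoff.
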(event `self.ReceiveTick`
  (params (DeltaSeconds :type "Float (single-precision)"))
  (bind _returnvalue_x (`KismetMathLibrary.BreakVector` (`SceneComponent.K2_GetComponentLocation` (`self.Ballards`))))
  ;[1 1 1] Moves Ballard
  (bind _speed (`self.GetSpeed`))
  (`self.K2_AddActorLocalTransform` (`KismetMathLibrary.MakeTransform` (`KismetMathLibrary.MakeVector` 0.0 _speed) (`KismetMathLibrary.MakeRotator` 0.0)))
  ;[1 1 1] Destroys obstacles when they move too far from the camera
  (if (< _returnvalue_x -20000.0)
    (`self.K2_DestroyActor`)))

(fn `GetSpeed`
  (returns (Speed :type "Float (double-precision)"))
  (bind _returnvalue (`GameplayStatics.GetActorOfClass` "/Game/Trevor/Road/BP_Road.BP_Road_C"))
  (return (`/Game/Trevor/Road/BP_Road.Speed` _returnvalue)))

(fn `UserConstructionScript`)