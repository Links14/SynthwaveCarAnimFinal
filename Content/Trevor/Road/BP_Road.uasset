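; BP_Road is a self-spawning, moving road segment that forms a continuous road with audio-linked street lamps.
; On BeginPlay it hands its SoundAnalyze reference to four child-actor street lamps and starts a one-shot timer.
; The timer spawns another BP_Road at the AttachPoint, passing SoundAnalyze along the chain.
; Tick slides each segment along local Y at a speed scaled by SeparateBPM, with no cleanup in this graph.
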(event `self.ReceiveBeginPlay`
  (bind _soundanalyze (`self.SoundAnalyze`))
  ;[1 1 1] Spawns More Road
  (`KismetSystemLibrary.K2_SetTimerDelegate` (delegate `Spawn Next Module`) (`self.Time`))
  (set `/Game/Trevor/Streetlight/BP_StreetLamp.SoundAnalyzerLamp` _soundanalyze (cast `/Game/Trevor/Streetlight/BP_StreetLamp` (`ChildActorComponent.ChildActor` (`self.BP_StreetLamp1`)) :!pure true))
  (set `/Game/Trevor/Streetlight/BP_StreetLamp.SoundAnalyzerLamp` _soundanalyze (cast `/Game/Trevor/Streetlight/BP_StreetLamp` (`ChildActorComponent.ChildActor` (`self.BP_StreetLamp2`)) :!pure true))
  (set `/Game/Trevor/Streetlight/BP_StreetLamp.SoundAnalyzerLamp` _soundanalyze (cast `/Game/Trevor/Streetlight/BP_StreetLamp` (`ChildActorComponent.ChildActor` (`self.BP_StreetLamp3`)) :!pure true))
  (set `/Game/Trevor/Streetlight/BP_StreetLamp.SoundAnalyzerLamp` _soundanalyze (cast `/Game/Trevor/Streetlight/BP_StreetLamp` (`ChildActorComponent.ChildActor` (`self.BP_StreetLamp4`)) :!pure true)))

(event `Spawn Next Module`
  (bind _attachpoint (`self.AttachPoint`))
  ;[1 1 1] Spawns More Road
  (`|SpawnActorFromClass` "BP_Road_C" (`KismetMathLibrary.MakeTransform` (`SceneComponent.K2_GetComponentLocation` _attachpoint) (`SceneComponent.K2_GetComponentRotation` _attachpoint)) "Undefined" "MultiplyWithRoot" null (`self.SoundAnalyze`) null))

(event `self.ReceiveTick`
  (params (DeltaSeconds :type "Float (single-precision)"))
  (`self.K2_AddActorLocalTransform` (`KismetMathLibrary.MakeTransform` (`KismetMathLibrary.MakeVector` 0.0 (* DeltaSeconds 99.5 (`self.SeparateBPM`))) (`KismetMathLibrary.MakeRotator` 0.0))))

(fn `UserConstructionScript`)